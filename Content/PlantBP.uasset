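; PlantBP is a plant hazard that damages the ThirdPersonCharacter while it overlaps the plant's SphereCollider.
; Begin overlap stores the character as Collisioner and sets IsHittingCharacter, and end overlap clears the flag.
; While the flag is set, Tick calls DoDamage with DamageAmount every frame, without scaling by delta time.
; An unconnected HitByDanger call never runs.
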(event OnComponentBeginOverlap(SphereCollider)
  (params (OverlappedComponent :type Primitive%20Component%20Object%20Reference) (OtherActor :type Actor%20Object%20Reference) (OtherComp :type Primitive%20Component%20Object%20Reference) (OtherBodyIndex :type Integer) (bFromSweep :type Boolean) (SweepResult :type Hit%20Result%20Structure%20%28by%20ref%29))
  (bind _asthird_person_character (Utilities|Casting|CastToThirdPersonCharacter OtherActor))
  (Variables|Default|SetisHittingCharacter true)
  (Variables|Default|Setcollisioner _asthird_person_character))

(event OnComponentEndOverlap(SphereCollider)
  (params (OverlappedComponent :type Primitive%20Component%20Object%20Reference) (OtherActor :type Actor%20Object%20Reference) (OtherComp :type Primitive%20Component%20Object%20Reference) (OtherBodyIndex :type Integer))
  (Utilities|Casting|CastToThirdPersonCharacter OtherActor)
  (Variables|Default|SetisHittingCharacter false))

(event EventBeginPlay)

(event Collision|EventActorBeginOverlap
  (params (OtherActor :type Actor%20Object%20Reference)))

(event EventTick
  (params (DeltaSeconds :type Float%20%28single-precision%29))
  (if (Variables|Default|GetisHittingCharacter)
    (Default|DoDamage (Variables|Default|Getcollisioner) (Variables|Default|GetdamageAmount))))

(fn ConstructionScript)